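; BP_Shot is a projectile actor in the Chaos Flesh MeatCube content whose static mesh acts as a collider for the flesh simulation.
; On BeginPlay it finds the BP_MeatManager and registers its StaticMeshComponent as a collider.
; When its Sphere hits anything other than its instigator, it deregisters the mesh from the manager and destroys itself.
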(event `self.ReceiveBeginPlay`
  ;[1 1 1] Register the static mesh component as a collider with the meat manager
  (bind _returnvalue (`GameplayStatics.GetActorOfClass` "/Game/ChaosFlesh/MeatCube/BP_MeatManager.BP_MeatManager_C"))
  (`/Engine/EditorBlueprintResources/StandardMacros.IsValid` _returnvalue
    (:`Is Valid`
      (`/Game/ChaosFlesh/MeatCube/BP_MeatManager.RegisterMeshComponent` _returnvalue (`self.StaticMeshComponent`)))))

(event `self.Sphere.OnComponentHit`
  (params (HitComponent :type "PrimitiveComponent Object Reference") (OtherActor :type "Actor Object Reference") (OtherComp :type "PrimitiveComponent Object Reference") (NormalImpulse :type "Vector Structure") (Hit :type "HitResult Structure (by ref)"))
  ;[1 1 1] When the component is being destroyed on collision, deregister it with the meat manager
  (if (!= (`self.GetInstigator`) OtherActor)
    (bind _returnvalue (`GameplayStatics.GetActorOfClass` "/Game/ChaosFlesh/MeatCube/BP_MeatManager.BP_MeatManager_C"))
    (`/Engine/EditorBlueprintResources/StandardMacros.IsValid` _returnvalue
      (:`Is Valid`
        (`/Game/ChaosFlesh/MeatCube/BP_MeatManager.RemoveMeshComponent` _returnvalue (`self.StaticMeshComponent`)))
      (:`Is Not Valid`
        _))
    (`self.K2_DestroyActor`)))

(fn `UserConstructionScript`)