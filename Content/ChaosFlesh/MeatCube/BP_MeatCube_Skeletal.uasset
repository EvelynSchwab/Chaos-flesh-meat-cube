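; Skeletal mesh meat cube actor that runs a Chaos Flesh deformable simulation rendered through an Optimus deformer graph.
; On BeginPlay it enables gameplay and collision components on the solver, then registers every static mesh actor and the player's flesh collider.
; It binds to BP_MeatManager to add or remove colliders at runtime.
; Tick feeds the SimToRender transform and Amount into the deformer instance.
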(event `self.ReceiveBeginPlay`
  (`self.StartSim`)
  ;[1 1 1] Bindings with the meat manager for registering static mesh elements for collision
  (bind _returnvalue (`GameplayStatics.GetActorOfClass` "/Game/ChaosFlesh/MeatCube/BP_MeatManager.BP_MeatManager_C"))
  (add `/Game/ChaosFlesh/MeatCube/BP_MeatManager.RemoveMeshComponent_Delegate` _returnvalue (`|CreateDelegate` :!event `RemoveMeshForCollision`))
  (add `/Game/ChaosFlesh/MeatCube/BP_MeatManager.RegisterMeshComponent_Delegate` _returnvalue (`|CreateDelegate` :!event `RegisterMeshForCollision`)))

(event `RegisterMeshForCollision`
  (params (Mesh :type "StaticMeshComponent Object Reference"))
  ;[1 1 1] Bindings with the meat manager for registering static mesh elements for collision
  (`DeformableCollisionsComponent.AddStaticMeshComponent` (`self.DeformableCollisions`) Mesh))

(event `RemoveMeshForCollision`
  (params (Mesh :type "StaticMeshComponent Object Reference"))
  ;[1 1 1] Bindings with the meat manager for registering static mesh elements for collision
  (`DeformableCollisionsComponent.RemoveStaticMeshComponent` (`self.DeformableCollisions`) Mesh))

(event `StartSim`
  ;[1 1 1] Init the meat cube
  (`SkinnedMeshComponent.SetMeshDeformer` (`self.SKM_MeatCube`) "/ChaosFlesh/Deformers/DG_FleshDeformer.DG_FleshDeformer")
  (`DeformablePhysicsComponent.EnableSimulation` (`self.DeformableGameplay`) (`self.DeformableSolver`))
  (`DeformablePhysicsComponent.EnableSimulation` (`self.DeformableCollisions`) (`self.DeformableSolver`))
  ;[1 1 1] Set up collisions with all static mesh actors and the player in the scene. This is obviously not a good thing to do in more complex scenes, and should be much more selective.
  (bind _outactors (`GameplayStatics.GetAllActorsOfClass` "/Script/Engine.StaticMeshActor"))
  (for _array_element _outactors
    (bind _asstatic_mesh_actor (cast `StaticMeshActor` _array_element))
    (`self.RegisterMeshForCollision` (`StaticMeshActor.StaticMeshComponent` _asstatic_mesh_actor)))
  (bind _asbp_third_person_character (cast `/Game/ThirdPerson/Blueprints/BP_ThirdPersonCharacter` (`GameplayStatics.GetPlayerCharacter` 0)))
  (`self.RegisterMeshForCollision` (`/Game/ThirdPerson/Blueprints/BP_ThirdPersonCharacter.FleshCollider` _asbp_third_person_character)))

(event `self.ReceiveTick`
  (params (DeltaSeconds :type "Float (single-precision)"))
  ;[1 1 1] Send sim data to the optimus deformer
  (bind _asoptimus_deformer_instance (cast `OptimusDeformerInstance` (`SkinnedMeshComponent.MeshDeformerInstance` (`self.SKM_MeatCube`))))
  (`OptimusDeformerInstance.SetTransformVariable` _asoptimus_deformer_instance "SimToRender" (`self.SimToRender`))
  (`OptimusDeformerInstance.SetFloatVariable` _asoptimus_deformer_instance "Amount" (`self.Amount`)))

(fn `UserConstructionScript`)